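; BP_EnemyBase is an enemy actor with health that deals contact damage to the first-person player on overlap.
; EnemyTakeDamage subtracts health, flashes a dynamic material parameter briefly via timer, and returns true on the killing hit.
; A Dying flag and DoOnce guard death, which stops projectile movement, disables collision, spawns an emitter and destroys the actor.
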(event `self.ReceiveBeginPlay`
  (bind _enemymesh (`self.EnemyMesh`))
  (bind _returnvalue (`PrimitiveComponent.CreateDynamicMaterialInstance` _enemymesh 0 (`PrimitiveComponent.GetMaterial` _enemymesh 0) "None"))
  (set `self.DynMaterial` _returnvalue))

(event `self.RootCollision.OnComponentBeginOverlap`
  (params (OverlappedComponent :type "PrimitiveComponent Object Reference") (OtherActor :type "Actor Object Reference") (OtherComp :type "PrimitiveComponent Object Reference") (OtherBodyIndex :type Integer) (bFromSweep :type Boolean) (SweepResult :type "HitResult Structure (by ref)"))
  (if (`self.ActorHasTag` OtherActor "Player")
    (bind _asbp_first_person_character (cast `/Game/FirstPerson/Blueprints/BP_FirstPersonCharacter` OtherActor))
    (`/Game/FirstPerson/Blueprints/BP_FirstPersonCharacter.RequestContactDamage` _asbp_first_person_character (`self.ContactDamage`))))

(event `HandleDeath`
  (`ActorComponent.Deactivate` (`self.ProjectileMovement`))
  (`PrimitiveComponent.SetCollisionEnabled` (`self.RootCollision`) "NoCollision")
  (`GameplayStatics.SpawnEmitterAtLocation` null (`self.K2_GetActorLocation`))
  (`self.K2_DestroyActor`))

(fn `EnemyTakeDamage`
  (params (Amount :type Integer) (ImpactPoint :type "Vector Structure"))
  (returns (bKilled :type Boolean))
  (if (`self.bDying`)
    (return false)
    (else
      (bind _output_get (set `self.Health` (- (`self.Health`) Amount)))
      (`self.Flash`)
      (if (<= _output_get 0)
        (`/Engine/EditorBlueprintResources/StandardMacros.DoOnce` false
          (:`Completed`
            (set `self.bDying` true)
            (`self.HandleDeath`)
            (return true)))
        (else
          (return false))))))

(fn `Flash`
  (`/Engine/EditorBlueprintResources/StandardMacros.IsValid` (`self.DynMaterial`)
    (:`Is Valid`
      (`MaterialInstanceDynamic.SetScalarParameterValue` (`self.DynMaterial`) "Flash" 1.0)
      (`KismetSystemLibrary.K2_SetTimer` null "ResetFlash" 0.05))
    (:`Is Not Valid`
      (return))))

(fn `ResetFlash`
  (`/Engine/EditorBlueprintResources/StandardMacros.IsValid` (`self.DynMaterial`)
    (:`Is Valid`
      (`MaterialInstanceDynamic.SetScalarParameterValue` (`self.DynMaterial`) "Flash" 0.0))
    (:`Is Not Valid`
      (return))))

(fn `UserConstructionScript`)