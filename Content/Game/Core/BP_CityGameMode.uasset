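; City game mode that tracks a shared city life pool and ends the game when it runs out.
; DecreaseCityLife clamps life, broadcasts the change and updates the HUD; the zero-life check runs only with a valid HUD.
; Game over fires once, pausing the game and swapping the HUD for a game-over widget with UI-only input.
; Bound handlers push normalized player health and city life to a HUD widget created outside this Blueprint.
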(event `self.ReceiveBeginPlay`
  (bind _asbp_first_person_character (cast `/Game/FirstPerson/Blueprints/BP_FirstPersonCharacter` (`GameplayStatics.GetPlayerPawn` 0)))
  (bind _output_get (set `self.PlayerRef` _asbp_first_person_character))
  (add `/Game/FirstPerson/Blueprints/BP_FirstPersonCharacter.OnPlayerHealthChanged` _output_get (delegate `Handle_PlayerHealthChanged`))
  (add `self.OnCityLifeChanged` (delegate `Handle_CityLifeChanged`))
  (set `self.CityLife` (`self.CityLifeMax`))
  (set `self.bGameOver` false)
  (add `self.OnGameOver` (delegate `ShowGameOverUI`)))

(event `Handle_PlayerHealthChanged`
  (params (CurrentHealth :type Integer) (MaxHealth :type Integer) (Ratio :type "Float (double-precision)"))
  (bind _hudwidget (`self.HUDWidget`))
  (`/Engine/EditorBlueprintResources/StandardMacros.IsValid` _hudwidget
    (:`Is Valid`
      (bind _output_get (set `self.HUDWidget` _hudwidget))
      (`/Game/UI/WBP_GameHUD.UpdatePlayerHealth` _output_get (`KismetMathLibrary.FClamp` (/ (`KismetMathLibrary.Conv_IntToDouble` CurrentHealth) (`KismetMathLibrary.Conv_IntToDouble` MaxHealth)))))))

(event `Handle_CityLifeChanged` :!signature `self.OnCityLifeChanged`
  (params (Current :type Integer) (Max :type Integer))
  (bind _hudwidget (`self.HUDWidget`))
  (`/Engine/EditorBlueprintResources/StandardMacros.IsValid` _hudwidget
    (:`Is Valid`
      (bind _output_get (set `self.HUDWidget` _hudwidget))
      (`/Game/UI/WBP_GameHUD.UpdateCityLife` _output_get (`KismetMathLibrary.FClamp` (/ (`KismetMathLibrary.Conv_IntToDouble` Current) (`KismetMathLibrary.Conv_IntToDouble` Max)))))))

(event `ShowGameOverUI`
  (bind _returnvalue (`GameplayStatics.GetPlayerController` 0))
  (bind _returnvalue_2 (`|CreateWidget` (`self.GameOverClass`) (`GameplayStatics.GetPlayerController` 0)))
  (bind _aswbp_game_over (cast `/Game/UI/WBP_GameOver` _returnvalue_2))
  (bind _output_get (set `self.GameOverWidget` _aswbp_game_over))
  (`UserWidget.AddToViewport` _output_get 0)
  (`Widget.RemoveFromParent` (`self.HUDWidget`))
  (`WidgetBlueprintLibrary.SetInputMode_UIOnlyEx` _returnvalue _output_get)
  (set `PlayerController.bShowMouseCursor` true _returnvalue))

(fn `DecreaseCityLife`
  (params (Amount :type Integer :default 1))
  (bind _citylifemax (`self.CityLifeMax`))
  (bind _hudwidget (`self.HUDWidget`))
  (if (`self.bGameOver`)
    (return)
    (else
      (bind _output_get (set `self.CityLife` (`KismetMathLibrary.Clamp` (- (`self.CityLife`) Amount) 0 (`self.CityLifeMax`))))
      (`self.OnCityLifeChanged` _output_get _citylifemax)
      (`/Engine/EditorBlueprintResources/StandardMacros.IsValid` _hudwidget
        (:`Is Valid`
          (`/Game/UI/WBP_GameHUD.UpdateCityLife` _hudwidget (`KismetMathLibrary.FClamp` (/ (`KismetMathLibrary.Conv_IntToDouble` _output_get) (`KismetMathLibrary.Conv_IntToDouble` _citylifemax))))
          (if (<= (`self.CityLife`) 0)
            (`self.HandleGameOver`)
            (else
              (return))))))))

(fn `GetCityLife`
  (returns (ReturnValue :type Integer))
  (return (`self.CityLife`)))

(fn `GetCityLifeMax`
  (returns (ReturnValue :type Integer))
  (return (`self.CityLifeMax`)))

(fn `HandleGameOver`
  (if (`self.bGameOver`)
    (return)
    (else
      (set `self.bGameOver` true)
      (`self.OnGameOver`)
      (`GameplayStatics.SetGamePaused` true))))

(fn `IsGameOver`
  (returns (ReturnValue :type Boolean))
  (return (`self.bGameOver`)))

(fn `UserConstructionScript`)