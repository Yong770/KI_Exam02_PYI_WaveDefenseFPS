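; Enemy spawner actor that periodically spawns EnemyClass actors while the city game is running.
; When StartOnBeginPlay is set, a looping timer calls SpawnOne, and the game mode's OnGameOver event clears it.
; SpawnOne spawns at a random X offset facing the ArrowSpawnDirection component, unless the game is over or AliveCount reaches MaxAliveLimit.
; AliveCount only increments here; nothing in this Blueprint decrements it.
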(event `self.ReceiveBeginPlay`
  (if (`self.bStartOnBeginPlay`)
    (bind _returnvalue (`KismetSystemLibrary.K2_SetTimer` null "SpawnOne" (`self.SpawnInterval`) true))
    (set `self.SpawnTimerHandle` _returnvalue)
    (bind _asbp_city_game_mode (cast `/Game/Game/Core/BP_CityGameMode` (`GameplayStatics.GetGameMode`)))
    (add `/Game/Game/Core/BP_CityGameMode.OnGameOver` _asbp_city_game_mode (delegate `OnGameOver_StopSpawning`))))

(event `OnGameOver_StopSpawning`
  (`KismetSystemLibrary.K2_ClearAndInvalidateTimerHandle` (`self.SpawnTimerHandle`))
  (`KismetSystemLibrary.PrintString` "Spawner Stopped"))

(fn `SpawnOne`
  (bind (_returnvalue_x _returnvalue_y _returnvalue_z) (`KismetMathLibrary.BreakVector` (`self.K2_GetActorLocation`)))
  (bind _asbp_city_game_mode (cast `/Game/Game/Core/BP_CityGameMode` (`GameplayStatics.GetGameMode`)))
  (if (`/Game/Game/Core/BP_CityGameMode.IsGameOver` _asbp_city_game_mode)
    (return)
    (elif (< (`self.AliveCount`) (`self.MaxAliveLimit`))
      (bind _returnvalue (`|SpawnActorFromClass` (`self.EnemyClass`) (`KismetMathLibrary.MakeTransform` (`KismetMathLibrary.MakeVector` (+ _returnvalue_x (`KismetMathLibrary.RandomFloatInRange` -1100.0 1100.0)) _returnvalue_y _returnvalue_z) (`SceneComponent.K2_GetComponentRotation` (`self.Arrow_SpawnDirection`))) "AdjustIfPossibleButAlwaysSpawn" "MultiplyWithRoot" null null))
      (set `self.SpawnedEnemy` _returnvalue)
      (set `self.AliveCount` (+ (`self.AliveCount`) 1))
      (`KismetSystemLibrary.PrintString` "Spawned!")
      (else
        (return)))))

(fn `UserConstructionScript`)